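; Player Blueprint that handles the pause menu, bound to the P key.
; P calls the Pause event with Visible, and a FlipFlop alternates that event between opening and closing branches.
; Opening creates WBP_Pause once, adds it to the viewport, shows the cursor and passes the player to its Setup.
; Both branches apply the caller's visibility argument, while closing also hides the cursor; game time is untouched.
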(event `Key|P`
  (params (Key :type "Key Structure"))
  (:`Pressed`
    (`self.Pause` "Visible")))

(event `Pause`
  (params (InVisibility :type "ESlateVisibility Enum" :default "Visible"))
  (bind _returnvalue (`GameplayStatics.GetPlayerController` 0))
  (bind _pause_hud (`self.Pause HUD`))
  (bind _pause_hud_2 (`self.Pause HUD`))
  (`/Engine/EditorBlueprintResources/StandardMacros.FlipFlop`
    (:`A`
      (`|ExecutionSequence`
        (:`then_0`
          (`/Engine/EditorBlueprintResources/StandardMacros.DoOnce` false
            (:`Completed`
              (bind _returnvalue_2 (`|CreateWidget` "/Game/UI/WBP_Pause.WBP_Pause_C" (`GameplayStatics.GetPlayerController` 0)))
              (set `self.Pause HUD` _returnvalue_2))))
        (:`then_1`
          (`Widget.SetVisibility` _pause_hud InVisibility)
          (set `PlayerController.bShowMouseCursor` true _returnvalue)
          (`UserWidget.AddToViewport` _pause_hud_2 0)
          (`/Game/UI/WBP_Pause.Setup` _pause_hud_2 self))))
    (:`B`
      (`Widget.SetVisibility` _pause_hud InVisibility)
      (set `PlayerController.bShowMouseCursor` false _returnvalue))))

(fn `UserConstructionScript`)