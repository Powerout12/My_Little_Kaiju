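; Enemy character that chases and attacks the player once PawnSensing spots them.
; Each sighting latches a seen flag and calls AI MoveTo toward the player; Tick halts movement until the first sighting.
; On arrival it turns to the player, spawns a projectile and applies damage directly.
; A half-second delay re-arms attacks, though every FollowPlayer call also re-arms them immediately.
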(event `self.ReceiveTick`
  (params (DeltaSeconds :type "Float (single-precision)"))
  (if (not (`self.IsSeeingPlayer`))
    (`MovementComponent.StopMovementImmediately` (`self.CharacterMovement`))))

(event `self.PawnSensing.OnSeePawn`
  (params (Pawn :type "Pawn Object Reference"))
  (set `self.IsSeeingPlayer` true)
  (`self.FollowPlayer`))

(event `FollowPlayer`
  (set `self.CanAttack` true)
  (if (`self.IsSeeingPlayer`)
    (`|AIMoveTo` self (0.0 0.0 0.0) (`GameplayStatics.GetPlayerCharacter` 0) 70.0
      (:`OnSuccess`
        (if (`self.CanAttack`)
          (set `self.CanAttack` false)
          (bind _asbp_player (cast `/Game/Blueprints/BP_Player` (`GameplayStatics.GetPlayerCharacter` 0)))
          (`self.K2_SetActorRotation` (`KismetMathLibrary.FindRelativeLookAtRotation` (`KismetMathLibrary.Conv_VectorToTransform` (`self.K2_GetActorLocation`)) (`self.K2_GetActorLocation` _asbp_player)))
          (`|SpawnActorFromClass` "/Game/Blueprints/BP_Projectile.BP_Projectile_C" (`SceneComponent.K2_GetComponentToWorld` (`self.SpawnProjectileLocation`)) "Undefined" "MultiplyWithRoot" null null)
          (`GameplayStatics.ApplyDamage` _asbp_player 1.0)
          (`KismetSystemLibrary.Delay` 0.5)
          (set `self.CanAttack` true))))
    (else
      (set `self.IsSeeingPlayer` false))))

(fn `UserConstructionScript`)