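; BP_Player is a click-to-move player with simple health tracking.
; On begin play it shows the mouse cursor, and a left click deprojects the cursor into a Visibility line trace, sending the controller to the hit point with SimpleMoveToLocation.
; Any damage reduces Health and prints it, with a "Game Over!" message at zero or below but no further death handling.
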(event `self.ReceiveBeginPlay`
  (set `PlayerController.bShowMouseCursor` true (`GameplayStatics.GetPlayerController` 0)))

(event `Key|LeftMouseButton`
  (params (Key :type "Key Structure"))
  (bind (_worldlocation _worlddirection) (`PlayerController.DeprojectMousePositionToWorld` (`GameplayStatics.GetPlayerController` 0)))
  (:`Pressed`
    (bind (_outhit _returnvalue) (`KismetSystemLibrary.LineTraceSingle` _worldlocation (+ _worldlocation (* _worlddirection 10000.0)) "TraceTypeQuery1"))
    (if _returnvalue
      (`AIBlueprintHelperLibrary.SimpleMoveToLocation` (`self.GetController`) (`.Location` (`GameplayStatics.BreakHitResult` _outhit))))))

(event `self.ReceiveAnyDamage`
  (params (Damage :type "Float (single-precision)") (DamageType :type "DamageType Object Reference") (InstigatedBy :type "Controller Object Reference") (DamageCauser :type "Actor Object Reference"))
  (bind _output_get (set `self.Health` (- (`self.Health`) Damage)))
  (`KismetSystemLibrary.PrintString` (`KismetStringLibrary.Conv_DoubleToString` _output_get))
  (if (<= (`self.Health`) 0.0)
    (`KismetSystemLibrary.PrintString` "Game Over!")))

(fn `UserConstructionScript`)